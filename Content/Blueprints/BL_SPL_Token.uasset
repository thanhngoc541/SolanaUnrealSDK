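; Demo Blueprint that exercises the SPL token lifecycle on Solana devnet when play begins.
; It creates and saves mint and recipient wallets, loads a payer wallet from file, and connects a Solana manager.
; It then creates the token, mints to the payer and transfers some to the recipient, each step gated on the previous success.
; Popups report successes, errors and the payer's balance after minting and transferring.
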(event `self.ReceiveBeginPlay`
  (bind (_errormessage _returnvalue) (`SolanaManager.CreateAndSaveWallet` "mint.json"))
  (bind _returnvalue_2 (`SolanaManager.GetPublicKey` _returnvalue))
  (`SolanaManager.DisplayKeyPair` _returnvalue "Mint Keypair")
  (bind (_errormessage_2 _returnvalue_3) (`SolanaManager.CreateAndSaveWallet` "receipient.json"))
  (bind _returnvalue_4 (`SolanaManager.GetPublicKey` _returnvalue_3))
  (`SolanaManager.DisplayKeyPair` _returnvalue_3 "receipient")
  (bind (_errormessage_3 _returnvalue_5) (`SolanaManager.LoadWalletFromFile` ""))
  (bind _returnvalue_6 (`SolanaManager.GetPublicKey` _returnvalue_5))
  (bind _returnvalue_7 (`SolanaManager.CreateSolanaManager`))
  (`SolanaManager.ConnectToSolana` _returnvalue_7 "https://api.devnet.solana.com")
  (bind (_errormessage_4 _returnvalue_8) (`SolanaManager.CreateSPLToken` _returnvalue_7 _returnvalue_5 _returnvalue))
  (if _returnvalue_8
    (`SolanaManager.ShowPopup` "Create SPL Token" "Success")
    (`SolanaManager.GetMintInfo` _returnvalue_7 _returnvalue_2)
    (bind (_errormessage_5 _returnvalue_9) (`SolanaManager.MintSPL` _returnvalue_7 _returnvalue_5 _returnvalue _returnvalue_6 1000000000000))
    (if _returnvalue_9
      (`SolanaManager.ShowPopup` "Mint SPL" "Success")
      (bind _balance (`SolanaManager.GetAssociatedTokenBalance` _returnvalue_7 _returnvalue_6 _returnvalue_2))
      (`SolanaManager.ShowPopup` "payer Token Balance" (`KismetStringLibrary.Conv_Int64ToString` _balance))
      (bind (_errormessage_6 _returnvalue_10) (`SolanaManager.TransferSPL` _returnvalue_7 _returnvalue_5 _returnvalue_4 _returnvalue_2 54000))
      (if _returnvalue_10
        (`SolanaManager.ShowPopup` "Transfered SPL" "Success")
        (bind _balance_2 (`SolanaManager.GetAssociatedTokenBalance` _returnvalue_7 _returnvalue_6 _returnvalue_2))
        (`SolanaManager.ShowPopup` "payer Token Balance" (`KismetStringLibrary.Conv_Int64ToString` _balance_2))
        (else
          (`SolanaManager.ShowPopup` "Transfer SPL Failed" _errormessage_6)))
      (else
        (`SolanaManager.ShowPopup` "Mint SPL Failed" _errormessage_5)))
    (else
      (`SolanaManager.ShowPopup` "Create SPL Token Failed" _errormessage_4))))

(fn `UserConstructionScript`)