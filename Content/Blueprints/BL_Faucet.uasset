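; BL_Faucet is an actor Blueprint that requests a Solana devnet faucet airdrop for a wallet when play begins.
; On BeginPlay it loads the wallet from file, shows its address, then connects a newly created Solana manager to the devnet RPC endpoint.
; The faucet request uses the wallet's public key, with popups reporting success or the error message and displaying the balance.
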(event `self.ReceiveBeginPlay`
  (bind (_errormessage _returnvalue) (`SolanaManager.LoadWalletFromFile` ""))
  (bind _returnvalue_2 (`SolanaManager.GetPublicKey` _returnvalue))
  (bind _returnvalue_3 (`SolanaManager.GetWalletAddress` _returnvalue))
  (`SolanaManager.ShowPopup` "Wallet Address" _returnvalue_3)
  (bind _returnvalue_4 (`SolanaManager.CreateSolanaManager`))
  (`SolanaManager.ConnectToSolana` _returnvalue_4 "https://api.devnet.solana.com")
  (bind (_errormessage_2 _returnvalue_5) (`SolanaManager.RequestFaucet` _returnvalue_4 _returnvalue_2 5000000000))
  (if _returnvalue_5
    (`SolanaManager.ShowPopup` "Request Faucet " "Success")
    (else
      (`SolanaManager.ShowPopup` "Request Faucet  Failed" _errormessage_2)))
  (bind _returnvalue_6 (`SolanaManager.GetWalletAddress` _returnvalue))
  (bind _balance (`SolanaManager.GetBalance` _returnvalue_4 _returnvalue_2))
  (`SolanaManager.ShowPopup` _returnvalue_6 _balance))

(fn `UserConstructionScript`)