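; Demo actor that runs a test SOL transfer on Solana devnet as soon as play begins.
; It loads the sender wallet from file, creates and saves a recipient wallet, and shows both addresses in popups.
; A Solana manager then connects to devnet and sends a hardcoded amount between them.
; Popups report either success with both resulting balances or the transfer's error message.
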(event `self.ReceiveBeginPlay`
  (bind (_errormessage _returnvalue) (`SolanaManager.LoadWalletFromFile` ""))
  (bind _returnvalue_2 (`SolanaManager.GetPublicKey` _returnvalue))
  (bind _returnvalue_3 (`SolanaManager.GetWalletAddress` _returnvalue))
  (`SolanaManager.ShowPopup` "Sender Address" _returnvalue_3)
  (bind (_errormessage_2 _returnvalue_4) (`SolanaManager.CreateAndSaveWallet` "receipient"))
  (bind _returnvalue_5 (`SolanaManager.GetPublicKey` _returnvalue_4))
  (bind _returnvalue_6 (`SolanaManager.GetWalletAddress` _returnvalue_4))
  (`SolanaManager.ShowPopup` "Receipient Address" _returnvalue_6)
  (bind _returnvalue_7 (`SolanaManager.CreateSolanaManager`))
  (`SolanaManager.ConnectToSolana` _returnvalue_7 "https://api.devnet.solana.com")
  (bind (_errormessage_3 _returnvalue_8) (`SolanaManager.TransferSOL` _returnvalue_7 _returnvalue _returnvalue_5 5400000))
  (if _returnvalue_8
    (`SolanaManager.ShowPopup` "Transfer SOL" "Success")
    (bind _balance (`SolanaManager.GetBalance` _returnvalue_7 _returnvalue_2))
    (`SolanaManager.ShowPopup` "Sender Sol Balance" _balance)
    (bind _balance_2 (`SolanaManager.GetBalance` _returnvalue_7 _returnvalue_5))
    (`SolanaManager.ShowPopup` "Receipient Balance" _balance_2)
    (else
      (`SolanaManager.ShowPopup` "Transfer SOL failed" _errormessage_3))))

(fn `UserConstructionScript`)